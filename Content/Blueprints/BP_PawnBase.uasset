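; Player pawn base for a lane-based game, sidestepping between lanes on Left and Right input while the level manager reports play.
; BeginPlay takes lane count and width from the level manager, starts near the middle lane and caches the EndCam-tagged actor.
; Timelines lerp the Y position, with a Moving flag and lane index guarding moves.
; GameStarted switches on smoke particles; HitObstacle spawns an explosion, hides the mesh and blends to the end camera.
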(event EventBeginPlay
  (bind (_levelmanager _levelmanagerfound) (CallFunction|GetLevelManager))
  ;[1 1 1] Initialize
  (if _levelmanagerfound
    (Variables|Default|SetLevelManagerRef _levelmanager)
    (Variables|Default|SetCurrentLength (+ (/ (Variables|/Game/Blueprints/GameMG/BP_LevelManager.BP_LevelManager_C|GetNumberofLanes (Variables|Default|GetLevelManagerRef)) 2) 1))
    (Variables|Default|SetLane%20Width (Variables|/Game/Blueprints/GameMG/BP_LevelManager.BP_LevelManager_C|GetLaneWidth (Variables|Default|GetLevelManagerRef)))
    (bind _outactors (Actor|GetAllActorswithTag "EndCam"))
    (Variables|Default|SetEndCam (Utilities|Array|Get(acopy) _outactors))
    (else
      (Development|PrintString "No LevelManager"))))

(event Input|ActionEvents|InputActionLeft
  (params (Key :type Key%20Structure :default "None"))
  (bind _returnvalue (Transformation|GetActorLocation))
  (:Pressed
    (if (Variables|/Game/Blueprints/GameMG/BP_LevelManager.BP_LevelManager_C|GetbIsPlaying (Variables|Default|GetLevelManagerRef))
      ;[1 1 1] Pressed Left whilst in Left most lane
      (if (not (<= (Variables|Default|GetCurrentLength) 1))
        (if (not (Variables|Default|GetbMoving))
          (Variables|Default|SetbMoving true)
          (Variables|Default|SetTargetPosition (- (.y (Transformation|GetActorLocation)) (Variables|Default|GetLane%20Width)))
          (bind _move (Timeline|MoveLeft PlayFromStart)
            (:Update
              (Transformation|SetActorLocation (Math|Vector|MakeVector (.x _returnvalue) (Math|Float|Lerp (.y _returnvalue) (Variables|Default|GetTargetPosition) _move) (.z _returnvalue)) false false))
            (:Finished
              (Variables|Default|SetbMoving false)
              (Math|Integer|DecrementInt (Variables|Default|GetCurrentLength)))))))))

(event Input|ActionEvents|InputActionRight
  (params (Key :type Key%20Structure :default "None"))
  (bind _returnvalue (Transformation|GetActorLocation))
  (:Pressed
    (if (Variables|/Game/Blueprints/GameMG/BP_LevelManager.BP_LevelManager_C|GetbIsPlaying (Variables|Default|GetLevelManagerRef))
      ;[1 1 1] Checando si presionamos derecha  cuando estamos en la derecha
      (if (not (== (Variables|Default|GetCurrentLength) (Variables|/Game/Blueprints/GameMG/BP_LevelManager.BP_LevelManager_C|GetNumberofLanes (Variables|Default|GetLevelManagerRef))))
        (if (not (Variables|Default|GetbMoving))
          (Variables|Default|SetbMoving true)
          (Variables|Default|SetTargetPosition (+ (.y (Transformation|GetActorLocation)) (Variables|Default|GetLane%20Width)))
          (bind _move (Timeline|MoveRight PlayFromStart)
            (:Update
              (Transformation|SetActorLocation (Math|Vector|MakeVector (.x _returnvalue) (Math|Float|Lerp (.y _returnvalue) (Variables|Default|GetTargetPosition) _move) (.z _returnvalue)) false false))
            (:Finished
              (Variables|Default|SetbMoving false)
              (Math|Integer|IncrementInt (Variables|Default|GetCurrentLength)))))))))

(fn ConstructionScript)

(fn HitObstacle
  (Components|DestroyComponent (Variables|Default|GetParticleSystem))
  (Effects|SpawnEmitteratLocation "/Game/MobileStarterContent/Particles/P_Explosion.P_Explosion" (Transformation|GetActorLocation))
  (Game|Player|SetViewTargetwithBlend (Game|GetPlayerController 0) (Variables|Default|GetEndCam) 2.0 "VTBlend_Linear" 0.0 false)
  (Rendering|ToggleVisibility (Variables|Default|GetPlayerMesh) false))

(fn GameStarted
  (Effects|Components|ParticleSystem|SetTemplate (Variables|Default|GetParticleSystem) "/Game/MobileStarterContent/Particles/P_Smoke.P_Smoke"))