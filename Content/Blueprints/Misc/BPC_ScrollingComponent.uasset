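; BPC_ScrollingComponent is an actor component that scrolls its owning actor while the level is playing.
; On BeginPlay it caches the level manager if one is found.
; Each Tick, while the manager reports IsPlaying, it offsets the owner by forward vector times the manager's LevelSpeed and delta time, without sweep.
; The world-space forward vector is applied as a local offset, so the owner's rotation affects the direction twice.
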(event EventBeginPlay
  (bind (_levelmanager _levelmanagerfound) (CallFunction|GetLevelManager))
  (if _levelmanagerfound
    (Variables|Default|SetLevelManagerRef _levelmanager)))

(event EventTick
  (params (DeltaSeconds :type Float%20%28single-precision%29))
  (bind _levelmanagerref (Variables|Default|GetLevelManagerRef))
  (Variables|Default|SetDelta%20Seconds DeltaSeconds)
  (Utilities|IsValid _levelmanagerref
    (:Is%20Valid
      (if (Variables|/Game/Blueprints/GameMG/BP_LevelManager.BP_LevelManager_C|GetbIsPlaying _levelmanagerref)
        (bind _output_get (Variables|Default|SetMovement (* (* (Transformation|GetActorForwardVector (Components|GetOwner)) (Variables|/Game/Blueprints/GameMG/BP_LevelManager.BP_LevelManager_C|GetLevelSpeed (Variables|Default|GetLevelManagerRef))) (Variables|Default|GetDelta%20Seconds))))
        (Transformation|AddActorLocalOffset (Components|GetOwner) _output_get false false)))))