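; BP_SpawnerFloor is a child spawner that builds a continuous floor from recycled tiles along the X axis.
; On BeginPlay it spawns tiles through the parent's SpawnActor, measures the first one's bounds for tile size, and chains the rest behind a tracked RearTile.
; When a tile hits the bounds, it moves to one tile length past RearTile and becomes the new rear, pooling tiles instead of respawning them.
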(event EventBeginPlay
  (|CallParentFunction)
  (for _index (range 0 (Variables|Default|GetActorsRequiredCount))
    (if (== _index 0)
      (bind _returnvalue (CallFunction|SpawnActor))
      (bind _output_get (Variables|Default|SetRearTile _returnvalue))
      (Variables|Default|SetTileSize (* (.x (.BoxExtent (Collision|GetActorBounds _returnvalue false false))) 2.0))
      (Transformation|SetActorLocationAndRotation _output_get (Transformation|GetActorLocation))
      (else
        (bind _returnvalue_2 (CallFunction|SpawnActor))
        (Transformation|SetActorLocation _returnvalue_2 (Math|Vector|MakeVector (+ (.x (Transformation|GetActorLocation (Variables|Default|GetRearTile))) (Variables|Default|GetTileSize)) (.y (Transformation|GetActorLocation (Variables|Default|GetRearTile))) 0.0) false false)
        (Variables|Default|SetRearTile _returnvalue_2)))))

(event EventSpawnActorHitBounds
  (params (OutBoundsActor :type Actor%20Object%20Reference))
  ;[1 1 1] Regresamos la pieza que alcanzo el final al inicio
  (|CallParentFunction 0)
  (Transformation|SetActorLocation OutBoundsActor (Math|Vector|MakeVector (+ (.x (Transformation|GetActorLocation (Variables|Default|GetRearTile))) (Variables|Default|GetTileSize)) (.y (Transformation|GetActorLocation (Variables|Default|GetRearTile))) (.z (Transformation|GetActorLocation (Variables|Default|GetRearTile)))) false false)
  (Variables|Default|SetRearTile OutBoundsActor))

(fn ConstructionScript
  (|CallParentFunction))

(fn SpawnActor
  (bind _returnvalue (|CallParentFunction))
  (return _returnvalue))