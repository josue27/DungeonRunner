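; Obstacle spawner that repeatedly places obstacles at its own location while the level is being played.
; On BeginPlay it looks up the level manager, then starts a self-recalling event that waits a random delay, spawns an obstacle and repeats while IsPlaying is true.
; Spawning is delegated to the parent spawner class, and actors reported as hitting the bounds are destroyed.
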(event Custom|LineUpObstacleSpawn
  (Utilities|FlowControl|Delay (Math|Random|RandomFloatinRange (Variables|Default|GetMinDelay) (Variables|Default|GetMaxDelay)))
  (CallFunction|PlaceObstacle)
  (if (Variables|/Game/Blueprints/GameMG/BP_LevelManager.BP_LevelManager_C|GetbIsPlaying (Variables|Default|GetLevel%20Manager%20Ref))
    (CallFunction|LineUpObstacleSpawn)))

(event EventBeginPlay
  (bind (_levelmanager _levelmanagerfound) (CallFunction|GetLevelManager))
  (if _levelmanagerfound
    (Variables|Default|SetLevel%20Manager%20Ref _levelmanager)
    (CallFunction|LineUpObstacleSpawn)))

(event EventSpawnActorHitBounds
  (params (OutBoundsActor :type Actor%20Object%20Reference))
  (Actor|DestroyActor OutBoundsActor))

(fn ConstructionScript
  (|CallParentFunction))

(fn PlaceObstacle
  (bind _returnvalue (CallFunction|SpawnActor))
  (Transformation|SetActorLocation _returnvalue (Transformation|GetActorLocation) false false))

(fn SpawnActor
  (bind _returnvalue (|CallParentFunction))
  (return _returnvalue))